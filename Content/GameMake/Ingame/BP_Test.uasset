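; BP_Test is a test actor that drives a Material Parameter Collection from its construction script.
; It writes Phase to the collection's first scalar parameter and the ColorA and ColorB entries selected by Set to the first two vector parameters.
; Parameters are looked up by index rather than name.
; The event graph is empty, and an older per-sphere dynamic material instance approach remains disconnected.
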(event EventBeginPlay)

(event Collision|EventActorBeginOverlap
  (params (OtherActor :type Actor%20Object%20Reference)))

(event EventTick
  (params (DeltaSeconds :type Float%20%28single-precision%29)))

(fn ConstructionScript
  (bind _collection (Variables|Default|GetCollection))
  (bind _set (Variables|Default|Getset))
  (bind _returnvalue (Class|MaterialParameterCollection|GetVectorParameterNames _collection))
  (Rendering|Material|SetScalarParameterValue _collection (Utilities|Array|Get(acopy) (Class|MaterialParameterCollection|GetScalarParameterNames _collection)) (Variables|Default|GetPhase) :!class /Script/Engine.KismetMaterialLibrary)
  (Rendering|Material|SetVectorParameterValue _collection (Utilities|Array|Get(acopy) _returnvalue) (Utilities|Array|Get(acopy) (Variables|Default|GetcolorA) _set) :!class /Script/Engine.KismetMaterialLibrary)
  (Rendering|Material|SetVectorParameterValue _collection (Utilities|Array|Get(acopy) _returnvalue 1) (Utilities|Array|Get(acopy) (Variables|Default|GetcolorB) _set) :!class /Script/Engine.KismetMaterialLibrary))